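; BP_Sparks is an actor that emits intermittent bursts from its PSparks component.
; BeginPlay starts an endless loop that waits a random few seconds, activates PSparks, then deactivates it after a very short delay.
; Each pass then applies a slight random world rotation to the component.
; It also reseeds a temporary random stream from real time, which the random calls do not use.
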(event `self.ReceiveBeginPlay`
  (bind _returnvalue (`KismetMathLibrary.RandomFloatInRange` 0.0 5.0))
  (bind _seconds (`GameplayStatics.GetAccurateRealTime`))
  (bind _p_sparks (`self.P_Sparks`))
  (`KismetSystemLibrary.Delay` _returnvalue :!label _label)
  (`ActorComponent.Activate` _p_sparks false)
  (`KismetSystemLibrary.Delay` 0.005)
  (`ActorComponent.Deactivate` _p_sparks)
  (`SceneComponent.K2_SetWorldRotation` (`self.P_Sparks`) (`KismetMathLibrary.MakeRotator` _returnvalue _returnvalue _returnvalue) false false)
  (`KismetMathLibrary.SetRandomStreamSeed` (`KismetMathLibrary.MakeRandomStream` _seconds) _seconds)
  (goto _label))

(fn `UserConstructionScript`)