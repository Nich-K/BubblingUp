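; BP_PoliceLight is a police light that flashes blue and red continuously from the moment play begins.
; BeginPlay runs an endless latent Delay chain that toggles Hidden In Game on the Blue and Red components, then wires back to its start.
; Each color double-flashes in turn, with a slightly longer pause before switching to the other.
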(event `self.ReceiveBeginPlay`
  (bind _blue (`self.Blue`))
  (bind _red (`self.Red`))
  (`SceneComponent.SetHiddenInGame` _blue false false :!label _label)
  (`KismetSystemLibrary.Delay` 0.1)
  (`SceneComponent.SetHiddenInGame` _blue true false)
  (`KismetSystemLibrary.Delay` 0.1)
  (`SceneComponent.SetHiddenInGame` _blue false false)
  (`KismetSystemLibrary.Delay` 0.1)
  (`SceneComponent.SetHiddenInGame` _blue true false)
  (`KismetSystemLibrary.Delay` 0.2)
  (`SceneComponent.SetHiddenInGame` _red false false)
  (`KismetSystemLibrary.Delay` 0.1)
  (`SceneComponent.SetHiddenInGame` _red true false)
  (`KismetSystemLibrary.Delay` 0.1)
  (`SceneComponent.SetHiddenInGame` _red false false)
  (`KismetSystemLibrary.Delay` 0.1)
  (`SceneComponent.SetHiddenInGame` _red true false)
  (`KismetSystemLibrary.Delay` 0.2)
  (goto _label))

(fn `UserConstructionScript`)