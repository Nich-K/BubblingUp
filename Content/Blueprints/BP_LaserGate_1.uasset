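; BP_LaserGate_1 is a laser gate actor that opens briefly when the G key is pressed, then closes itself.
; BeginPlay enables input for the first player controller and starts the looping gate sound.
; G stops the loop and swaps the closed component for the open one, disabling the closed component's collision.
; After timed delays, it plays GateOpenSound while restoring the closed state, then restarts the loop.
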(event `Key|G`
  (params (Key :type "Key Structure"))
  (bind _gate_closed (`self.Gate_closed`))
  (bind _gate_closed_2 (`self.Gate_closed`))
  (:`Pressed`
    (`KismetSystemLibrary.PrintString` "Hello")
    ;[1 1 1] Gate opens
    (`AudioComponent.Stop` (`self.Gate_Loop`))
    (`SceneComponent.SetHiddenInGame` (`self.Gate_open`) false false)
    (`SceneComponent.SetHiddenInGame` _gate_closed_2 true false)
    (`PrimitiveComponent.SetCollisionEnabled` _gate_closed_2 "NoCollision")
    (`KismetSystemLibrary.Delay` 1.0)
    ;[1 1 1] Gate closes
    (`AudioComponent.Play` (`self.Gate_Open_Sound`) 0.0)
    (`SceneComponent.SetHiddenInGame` (`self.Gate_open`) true false)
    (`SceneComponent.SetHiddenInGame` _gate_closed false false)
    (`PrimitiveComponent.SetCollisionEnabled` _gate_closed "QueryAndPhysics")
    (`KismetSystemLibrary.Delay` 5.63)
    (`AudioComponent.Play` (`self.Gate_Loop`) 0.0)))

(event `self.ReceiveBeginPlay`
  ;[1 1 1] Start
  (`self.EnableInput` (`GameplayStatics.GetPlayerController` 0))
  (`AudioComponent.Play` (`self.Gate_Loop`) 0.0))

(fn `UserConstructionScript`)